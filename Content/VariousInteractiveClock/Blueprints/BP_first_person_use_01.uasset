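; First-person player Blueprint that detects and uses interactive BP_XHC_Use objects and manages camera depth of field.
; Looping timers sphere-trace to update use-icon validity and notify looked-at objects, and line-trace to compute focus distance and set aperture.
; Use and AlternativeUse inputs line-trace on the Camera channel, then call enabled targets.
; The construction script adds a custom-depth highlight post-process material; empty OtherUses and FocalDistance events serve as hooks.
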(event `self.ReceiveBeginPlay`
  ;[0 0.5156 0.1942] Automatic settings at the beginning of each game
  (`self.EventBegin01`))

(event `LoadComponent01`
  ;[0 0.5156 0.1942] Automatic settings at the beginning of each game
  (`self.LoadComponent`))

(event `EventBegin01`
  ;[0 0.5156 0.1942] Automatic settings at the beginning of each game
  (`self.EventBegin`)
  (bind _returnvalue (`|CreateWidget` "/Game/VariousInteractiveClock/Widget/WI_UseIconHUD.WI_UseIconHUD_C"))
  (bind _output_get (set `self.EyeHUD` _returnvalue))
  (`UserWidget.AddToViewport` _output_get 0)
  (`self.LoadComponent01`)
  (`KismetSystemLibrary.K2_SetTimer` null "Update Use Icon" 0.1 true) ; Judgment interaction
  (`KismetSystemLibrary.K2_SetTimer` null "Update DOF" 0.05 true) ; Update depth of field
)

(event `UseHitActor`
  ;[1 1 0] Use Settings.(Determine if the object is interactive and pass the data to the child)
  (bind _hitactor (`self.GetUseable`))
  (bind _asbp_xhc_use (cast `/Game/VariousInteractiveClock/Blueprints/BP_XHC_Use` _hitactor))
  (if (`/Game/VariousInteractiveClock/Blueprints/BP_XHC_Use.InteractionEnabled` _asbp_xhc_use)
    (`/Game/VariousInteractiveClock/Blueprints/BP_XHC_Use.Use` _asbp_xhc_use false)))

(event `AlternativeUseHitActor`
  ;[1 1 0] Use Settings.(Determine if the object is interactive and pass the data to the child)
  (bind _hitactor (`self.GetUseable`))
  (bind _asbp_xhc_use (cast `/Game/VariousInteractiveClock/Blueprints/BP_XHC_Use` _hitactor))
  (if (`/Game/VariousInteractiveClock/Blueprints/BP_XHC_Use.InteractionEnabled` _asbp_xhc_use)
    (`self.OtherUses` _hitactor)
    (`/Game/VariousInteractiveClock/Blueprints/BP_XHC_Use.AlternativeUse` _asbp_xhc_use false)))

(event `OtherUses`
  (params (Actor :type "Actor Object Reference"))
  ;[0.8224 0 1] Standby
)

(event `FocalDistance`
  ;[0.8224 0 1] Standby
)

(event `InputAction|Use` :overrideparent false
  (params (Key :type "Key Structure"))
  ;[1 1 1] Input Settings
  (:`Pressed`
    (`self.UseHitActor`)))

(event `InputAction|AlternativeUse` :overrideparent false
  (params (Key :type "Key Structure"))
  ;[1 1 1] Input Settings
  (:`Pressed`
    (`self.AlternativeUseHitActor`)))

(event `Off_light_whenfocus`
  ;[1 1 1] FOCUS lights
  (`SceneComponent.SetHiddenInGame` (`self.Lights`) true true))

(event `On_light_whenfocus`
  ;[1 1 1] FOCUS lights
  (`SceneComponent.SetHiddenInGame` (`self.Lights`) false true))

(fn `Update DOF`
  (bind _firstpersoncamera (`self.FirstPersonCamera`))
  (bind _output_get (set `self.FocusEndLine` (+ (* (`SceneComponent.GetForwardVector` _firstpersoncamera) (`self.MaxFocusDistance`)) (0.0 0.0 0.0))))
  (bind (_outhit _returnvalue) (`KismetSystemLibrary.LineTraceSingle` (`SceneComponent.K2_GetComponentLocation` _firstpersoncamera) _output_get "TraceTypeQuery1" true)) ; If the camera channel is used, it will be blocked by the touchharea of use
  (if _returnvalue
    (bind (_bblockinghit _binitialoverlap _time _distance _location _impactpoint _normal _impactnormal _physmat) (`GameplayStatics.BreakHitResult` _outhit))
    (if (== _physmat null)
      (set `self.FocusLocation` (`self.MaxFocusDistance`) :!label _label)
      (else
        (set `self.FocusLocation` (`KismetMathLibrary.VSize` (- _location (`SceneComponent.K2_GetComponentLocation` (`self.FirstPersonCamera`)))))))
    (else
      (goto _label)))
  (setmembers `PostProcessSettings` :`StructRef` (`CameraComponent.PostProcessSettings` (`self.FirstPersonCamera`)) :`DepthOfFieldFstop` (select `bool` (`self.Inspecting`) :`false` (`self.DOF Aperture`) :`true` (`self.CurrentAperture(Inspecting)`)))
  (`self.FocalDistance`))

(fn `Update Use Icon`
  (bind _firstpersoncamera (`self.FirstPersonCamera`))
  (bind _returnvalue (`SceneComponent.K2_GetComponentLocation` _firstpersoncamera))
  ;[1 1 1] Determine if the mouse can interact and update the Use Icon
  (if (not (`self.HideUseIcon`))
    (`|ExecutionSequence`
      (:`then_0`
        (bind _outactors (`GameplayStatics.GetAllActorsWithTag` "IgnoreTrace"))
        (bind (_outhit _returnvalue_2) (`KismetSystemLibrary.SphereTraceSingle` _returnvalue (+ _returnvalue (* (`SceneComponent.GetForwardVector` _firstpersoncamera) (`self.UseDistance`))) 1.0 "TraceTypeQuery2" false _outactors)) ; Expanding the sphere range with other useful center points, only interactive objects, using camera channels
        (bind (_bblockinghit _binitialoverlap _time _distance _location _impactpoint _normal _impactnormal _physmat _hitactor _hitcomponent) (`GameplayStatics.BreakHitResult` _outhit))
        (bind _asbp_xhc_use (cast `/Game/VariousInteractiveClock/Blueprints/BP_XHC_Use` _hitactor)
          (:`then`
            (set `self.UseableValid` (and (`/Game/VariousInteractiveClock/Blueprints/BP_XHC_Use.InteractionEnabled` _asbp_xhc_use) (`KismetSystemLibrary.IsValid` _hitcomponent) _returnvalue_2))
            (`/Game/VariousInteractiveClock/Blueprints/BP_XHC_Use.Looked_at` _asbp_xhc_use))
          (:`CastFailed`
            (set `self.UseableValid` false) ; Not hit actor
          )))
      (:`then_1`
        (if (`self.Dead`)
          (`self.DisableInput` (`GameplayStatics.GetPlayerController` 0))
          (set `self.Running` false))))))

(fn `UserConstructionScript`
  (bind _array (break `WeightedBlendables` (`.WeightedBlendables` (break `PostProcessSettings` (`CameraComponent.PostProcessSettings` (`self.FirstPersonCamera`))))))
  (`parent.UserConstructionScript`)
  ;[1 0.3482 0.0546] Project Settings>>Engine -Rendering>>Postprocessing>>Custom Depth-Stencil Pass>>Enabled with Stencil
  (bind _returnvalue (`KismetMaterialLibrary.CreateDynamicMaterialInstance` "/Game/VariousInteractiveClock/Materials/MI_PP_highlightShelter.MI_PP_highlightShelter" "Highlight"))
  (bind _output_get (set `self.Highlight` _returnvalue))
  (`MaterialInstanceDynamic.SetScalarParameterValue` _output_get "CustomDepth ID" (`KismetMathLibrary.Conv_IntToDouble` (`self.CustomDepth ID`)))
  (`KismetArrayLibrary.Array_Set` _array (`KismetArrayLibrary.Array_Length` _array) (make `WeightedBlendable` 1.0 _output_get) true))