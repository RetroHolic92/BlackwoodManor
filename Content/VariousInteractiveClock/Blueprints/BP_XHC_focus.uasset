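; Base interactable for close-up inspection in the interactive clock set, moving the player's first-person camera to an EyeCapture view.
; A timeline blends camera transform, FOV and DOF aperture while inspection lights fade in, then a looping timer locks the camera to the view.
; Ending inspection reverses the timelines and restores player input, lights and camera.
; Empty events like InspectionUse, ClockStart and PutBack serve as hooks for specific behavior.
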(event `self.ReceiveBeginPlay`
  (`parent.ReceiveBeginPlay`))

(event `InputAction|Use`
  (params (Key :type "Key Structure"))
  ;[1 1 1] Input Settings
  (:`Pressed`
    (`self.InspectionUse`)))

(event `InputAction|AlternativeUse`
  (params (Key :type "Key Structure"))
  ;[1 1 1] Input Settings
  (:`Pressed`
    (`self.InspectionAlternativeUse`)))

(event `UpdateInspectionTimeline`
  (bind _player (`self.player`))
  ;[1 1 1] Inspection Timeline Update
  (`SceneComponent.K2_SetWorldTransform` (`/Game/VariousInteractiveClock/Blueprints/BP_first_person_base.FirstPersonCamera` (`self.player`)) (`KismetMathLibrary.TLerp` (`self.eyeWorldTransform`) (select `ETimelineDirection` (`self.AnimationDirection`) :`Forward` (`SceneComponent.K2_GetComponentToWorld` (`self.EyeCapture`)) :`Backward` (`self.eyeCurrentTransform`)) (`self.AnimationValue`)) false false)
  (`CameraComponent.SetFieldOfView` (`/Game/VariousInteractiveClock/Blueprints/BP_first_person_base.FirstPersonCamera` (`self.player`)) (`KismetMathLibrary.Lerp` (select `ETimelineDirection` (`self.AnimationDirection`) :`Forward` (`self.Current FOV`) :`Backward` (`/Game/VariousInteractiveClock/Blueprints/BP_first_person_base.DefaultView` (`self.player`))) (`self.InspectionViewFOV`) (`self.AnimationValue`)))
  (set `/Game/VariousInteractiveClock/Blueprints/BP_first_person_use_01.CurrentAperture(Inspecting)` (`KismetMathLibrary.Lerp` (`/Game/VariousInteractiveClock/Blueprints/BP_first_person_use_01.DOF Aperture` _player) (`/Game/VariousInteractiveClock/Blueprints/BP_first_person_use_01.DOF Aperture (Inspecting)` _player) (`self.AnimationValue`)) _player))

(event `BeginInspection`
  (params (focusactor :type "SceneComponent Object Reference"))
  (bind _player (`self.player`))
  ;[0.4069 1 0.07339] Begin Inspection
  (if (`self.CanInspection`)
    (`self.SetPlayer`)
    (`/Game/VariousInteractiveClock/Blueprints/BP_first_person_use_01.Off_light_whenfocus` (`self.player`))
    (set `self.focusactor` focusactor)
    (`self.Player Input` false)
    (set `/Game/VariousInteractiveClock/Blueprints/BP_first_person_use_01.XhcFocusRef` self _player)
    (bind _output_get (set `/Game/VariousInteractiveClock/Blueprints/BP_first_person_use_01.Inspecting` true _player))
    (set `self.Inspecting` _output_get)
    (set `self.InspectMoving` true)
    (set `self.BeginFocus` true)
    (bind _output_get_2 (set `self.eyeWorldTransform` (`SceneComponent.K2_GetComponentToWorld` (`/Game/VariousInteractiveClock/Blueprints/BP_first_person_base.FirstPersonCamera` (`self.player`)))))
    (`SceneComponent.K2_SetWorldTransform` (`self.PlayerEyeInitial`) _output_get_2 false false)
    (`self.Sign Invisible`)
    (`KismetSystemLibrary.Delay` 0.1)
    (`/Game/VariousInteractiveClock/Blueprints/BP_first_person_base.ShakeheardT_stop` (`self.player`))
    (`self.PlayInspectionTimeline`)))

(event `PlayInspectionTimeline`
  (bind _player (`self.player`))
  ;[1 1 1] Animation of the perspective rotating with the object during inspection timeline.
  (set `self.lightslocation` (.location (`SceneComponent.GetRelativeTransform` (`/Game/VariousInteractiveClock/Blueprints/BP_first_person_use_01.Lights` (`self.player`)))))
  (`self.Sign Invisible`)
  (`self.InspectionLightOn`)
  (`SceneComponent.K2_SetRelativeLocation` (`/Game/VariousInteractiveClock/Blueprints/BP_first_person_use_01.Lights` (`self.player`)) (+ (`self.lightslocation`) (0.0 0.0 -20.0)) false false)
  (set `self.player to eye` (`self.transform-` (`self.GetTransform` (`self.player`)) (`SceneComponent.K2_GetComponentToWorld` (`/Game/VariousInteractiveClock/Blueprints/BP_first_person_base.FirstPersonCamera` (`self.player`)))))
  (set `/Game/VariousInteractiveClock/Blueprints/BP_first_person_base.PauseRun` true _player)
  (`TimelineComponent.Stop` (`/Game/VariousInteractiveClock/Blueprints/BP_first_person_base.viewTimeline` _player))
  (set `self.Current FOV` (`CameraComponent.FieldOfView` (`/Game/VariousInteractiveClock/Blueprints/BP_first_person_base.FirstPersonCamera` _player)))
  (bind (_direction _animation) (`Timeline|Inspection Timeline` :!via `PlayFromStart` :!label _label)
    (:`Update`
      (set `self.AnimationDirection` _direction)
      (set `self.AnimationValue` _animation)
      (`self.UpdateInspectionTimeline`))
    (:`Finished`
      (`self.FinishedInspectionTimeline`)
      (set `self.InspectMoving` false))))

(event `StopInspectionTimeline`
  ;[1 1 1] Animation of the perspective rotating with the object during inspection timeline.
  (goto _label :!via `Stop`))

(event `EndInspection`
  (params (ReverseFromCurrent :type Boolean))
  ;[1 0 0.3215] End Inspection
  (`/Engine/EditorBlueprintResources/StandardMacros.IsValid` (`self.player`) ; Not adding this item may cause a bug when moving
    (:`Is Valid`
      (`self.ControllerInput` false)
      (set `self.BeginFocus` false)
      (`KismetSystemLibrary.K2_ClearTimer` null "PlayerFollowFocus")
      (set `self.eyeWorldTransform` (`SceneComponent.K2_GetComponentToWorld` (`self.PlayerEyeInitial`)))
      (set `self.eyeCurrentTransform` (`SceneComponent.K2_GetComponentToWorld` (`/Game/VariousInteractiveClock/Blueprints/BP_first_person_base.FirstPersonCamera` (`self.player`))))
      (`self.SetPlayer`)
      (bind _output_get (set `/Game/VariousInteractiveClock/Blueprints/BP_first_person_use_01.Inspecting` (not ReverseFromCurrent) (`self.player`)))
      (set `self.Inspecting` _output_get)
      (`self.ReverseInspectionTimeline` ReverseFromCurrent))))

(event `FinishedInspectionTimeline`
  (bind _player (`self.player`))
  ;[1 1 1] Finished Inspection Timeline (After automatic rotation of the actor)
  (switch `ETimelineDirection` (`self.AnimationDirection`) ; Controlled by Inspection Timeline
    (:`Forward`
      (`KismetSystemLibrary.K2_SetTimer` null "PlayerFollowFocus" 0.015 true)
      (`self.ControllerInput` true)
      (if (`self.DisplayCursor`)
        (`self.MouseSetting` true))
      (`self.StartInspect`))
    (:`Backward`
      (`self.HideInspectionWidget`)
      (`self.Player Input` true)
      (bind _output_get (set `/Game/VariousInteractiveClock/Blueprints/BP_first_person_use_01.Inspecting` false (`self.player`)))
      (set `self.Inspecting` _output_get)
      (set `/Game/VariousInteractiveClock/Blueprints/BP_first_person_base.PauseRun` false (`self.player`))
      (`self.UpdateSignDisplay`)
      (`SceneComponent.K2_SetRelativeLocation` (`/Game/VariousInteractiveClock/Blueprints/BP_first_person_use_01.Lights` (`self.player`)) (`self.lightslocation`) false false)
      (`/Game/VariousInteractiveClock/Blueprints/BP_first_person_use_01.On_light_whenfocus` (`self.player`))
      (`self.PutBack`)
      (`SceneComponent.K2_SetRelativeTransform` (`/Game/VariousInteractiveClock/Blueprints/BP_first_person_base.FirstPersonCamera` _player) (`/Game/VariousInteractiveClock/Blueprints/BP_first_person_base.Eye_transform` _player) false false) ; Reset eye default position
      (if (and (`self.InteractionEnabled`) (`self.Show_sign`))
        (if (`PrimitiveComponent.IsOverlappingActor` (`self.SignArea`) (`self.player`))
          (`self.Sign Visible`)
          (else
            (`self.Sign Invisible`)))
        (else
          (`self.Sign Invisible`))))))

(event `ReverseInspectionTimeline`
  (params (ReverseFromCurrent :type Boolean))
  (bind _player_to_eye (`self.player to eye`))
  (bind _eyeworldtransform (`self.eyeWorldTransform`))
  (bind (_a_b_location _a_b_rotation) (`KismetMathLibrary.BreakTransform` (`self.transform+` _player_to_eye _eyeworldtransform)))
  (bind (_returnvalue_roll _returnvalue_pitch _returnvalue_yaw) (`KismetMathLibrary.BreakRotator` (`KismetMathLibrary.NormalizedDeltaRotator` _a_b_rotation (`self.K2_GetActorRotation` (`self.player`)))))
  ;[1 1 1] Animation of the perspective rotating with the object during inspection timeline.
  (`|ExecutionSequence`
    (:`then_0`
      (`Pawn.AddControllerYawInput` (`self.player`) (/ _returnvalue_yaw 2.5))
      (`self.K2_SetActorTransform` (`self.player`) (`self.transform+` _player_to_eye _eyeworldtransform) false false)
      (`self.InspectionLightOff`))
    (:`then_1`
      (if (`self.DisplayCursor`)
        (`self.MouseSetting` false))
      (if ReverseFromCurrent
        (goto _label :!via `Reverse`)
        (else
          (goto _label :!via `ReverseFromEnd`))))))

(event `ZoomIn`
  ;[1 0 0.9435] Standby
)

(event `ExamineItem`
  ;[1 0 0.9435] Standby
)

(event `InspectionUse`
  ;[1 0 0.9435] Standby
)

(event `UseInventoryItem`
  ;[1 0 0.9435] Standby
)

(event `InspectionLightOn`
  (bind (_cache_r _cache_g) (break `LinearColor` (`self.Cache`)))
  (bind _cache_r_2 (break `LinearColor` (`self.Cache`)))
  ;[1 1 1] Animation of the perspective rotating with the object during inspection timeline.
  (`SceneComponent.SetVisibility` (`self.InspectionLight`) true false)
  (`SceneComponent.SetVisibility` (`self.InspectionLight2`) true false)
  (bind (_direction _animation) (`Timeline|InspectionLightTimeline` :!via `PlayFromStart` :!label _label_2)
    (:`Update`
      (`LightComponent.SetIntensity` (`self.InspectionLight`) (`KismetMathLibrary.Lerp` 0.0 _cache_r_2 _animation))
      (`LightComponent.SetIntensity` (`self.InspectionLight2`) (`KismetMathLibrary.Lerp` 0.0 _cache_g _animation)))
    (:`Finished`
      (switch `ETimelineDirection` _direction
        (:`Backward`
          (`SceneComponent.SetVisibility` (`self.InspectionLight`) false false)
          (`SceneComponent.SetVisibility` (`self.InspectionLight2`) false false))))))

(event `InspectionAlternativeUse`
  ;[1 0 0.9435] Standby
)

(event `HideInspectionWidget`
  ;[1 0 0.9435] Standby
)

(event `InventoryUse`
  ;[1 0 0.9435] Standby
)

(event `Zoom Out`
  ;[1 0 0.9435] Standby
)

(event `InspectionLightOff`
  ;[1 1 1] Animation of the perspective rotating with the object during inspection timeline.
  (goto _label_2 :!via `ReverseFromEnd`))

(event `Shake`
  (params (ShakeValue :type "Float (double-precision)"))
  ;[1 0 0.9435] Standby
)

(event `ClockStart`
  ;[1 0 0.9435] Standby
)

(event `StartInspect`
  ;[1 0 0.9435] Standby
)

(event `ClockPause`
  ;[1 0 0.9435] Standby
)

(event `PutBack`
  ;[1 0 0.9435] Standby
)

(event `ClockStop`
  ;[1 0 0.9435] Standby
)

(fn `PlayerFollowFocus`
  (`SceneComponent.K2_SetWorldTransform` (`/Game/VariousInteractiveClock/Blueprints/BP_first_person_base.FirstPersonCamera` (`self.player`)) (`SceneComponent.K2_GetComponentToWorld` (`self.EyeCapture`)) false false))

(fn `UserConstructionScript`
  (bind _returnvalue (select `bool` (`self.InspectionAnimation`) :`false` 0.001 :`true` (`self.InspectionAnimationSpeed (Sec)`)))
  (`parent.UserConstructionScript`)
  (if (`self.InteractionEnabled`)
    (`self.PlayRate` (`self.Inspection Timeline`) _returnvalue)
    (`self.PlayRate` (`self.InspectionLightTimeline`) _returnvalue)
    (set `self.Cache` (make `LinearColor` (`LightComponentBase.Intensity` (`self.InspectionLight`)) (`LightComponentBase.Intensity` (`self.InspectionLight2`)) 0.0 1.0))
    (else
      (set `self.InspectionAnimation` false)
      (set `self.InspectionAnimationSpeed (Sec)` 0.0)
      (set `self.DisplayCursor` false))))