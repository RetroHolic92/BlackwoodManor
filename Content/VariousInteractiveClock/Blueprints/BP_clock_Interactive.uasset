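; Interactive clock actor with optional second hand, base and swinging pendulum, inspectable through a WI_function widget that receives its time and alarm values.
; A looping timer scaled by Speed runs UpdateTime, using system time, a moving second hand only, or a simulated one-second step.
; SetClockHand rotates the hand pivots and triggers hourly chimes or the alarm, while the MovePendulum timeline drives swing and tick sounds.
; The construction script previews the hands and reconciles conflicting options.
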(event `self.ReceiveBeginPlay`
  (`self.update`)
  (`self.Creat UI`))

(event `Creat UI`
  (bind _returnvalue (`|CreateWidget` "/Game/VariousInteractiveClock/Widget/WI_function.WI_function_C" null self))
  (bind _output_get (set `self.WI_function` _returnvalue))
  (`WidgetComponent.SetWidget` (`self.function`) _output_get)
  (`SceneComponent.SetVisibility` (`self.function`) false true))

(event `self.Use`
  (params (`XHC Event` :type Boolean))
  ;[1 0.04588 0] Child blueprint essential
  (`self.BeginInspection` (`self.Billboard`))
  (`UserWidget.AddToViewport` (`self.WI_function`) 100)
  (`/Game/VariousInteractiveClock/Widget/WI_function.ClockFocStart` (`self.WI_function`))
  (`/Game/VariousInteractiveClock/Widget/WI_function.Initial Time` (`self.WI_function`) (`self.Hour`) (`self.Min`) (`self.Sec`))
  (`/Game/VariousInteractiveClock/Widget/WI_function.Alarm Time` (`self.WI_function`) (`self.hour_alarm`) (`self.min_alarm`) (`self.sec_alarm`)))

(event `self.InspectionAlternativeUse`
  ;[1 0.04588 0] Child blueprint essential
  (`/Game/VariousInteractiveClock/Widget/WI_function.ClockFocStop` (`self.WI_function`))
  (`KismetSystemLibrary.Delay` 0.5)
  (`self.EndInspection` false)
  (`Widget.RemoveFromParent` (`self.WI_function`)))

(event `Upload`
  ;[1 1 1] Upload
  (`self.Set Clock Hand` (`self.Sec`) (`self.Min`) (`self.Hour`)))

(event `UpDate`
  (bind _returnvalue (`KismetMathLibrary.Now`))
  (bind _pendulum_pivot (`self.pendulum_pivot`))
  (bind _pendulum_pivot_2 (`self.pendulum_pivot`))
  (bind _returnvalue_2 (`SceneComponent.GetRelativeTransform` _pendulum_pivot))
  (bind _returnvalue_3 (`SceneComponent.GetRelativeTransform` _pendulum_pivot_2))
  ;[1 1 1] Update time
  (if (`self.AutoWorking`)
    (set `self.0_hour` (- (`self.Hour`) (`KismetMathLibrary.GetHour` _returnvalue)))
    (set `self.0_min` (- (`self.Min`) (`KismetMathLibrary.GetMinute` _returnvalue)))
    (set `self.0_sec` (- (`self.Sec`) (`KismetMathLibrary.GetSecond` _returnvalue)))
    (`self.UpdateSpeed`)
    (else
      (`|ExecutionSequence`
        (:`then_0`
          (bind (_direction _2s) (`Timeline|MovePendulum` :!via `Stop` :!label _label)
            (:`Update`
              (`SceneComponent.K2_SetRelativeRotation` _pendulum_pivot (`KismetMathLibrary.MakeRotator` (.roll (.rotation _returnvalue_2)) (* (`self.Angle Pendulum`) _2s) (.yaw (.rotation _returnvalue_2))) false false))
            (:`clock ticking`
              (`GameplayStatics.SpawnSoundAttached` (`self.TickSound`) (`self.clock`) "None" (0.0 0.0 0.0) (struct) "KeepRelativeOffset" true (`self.Volume`) 1.0 0.0 (`self.SoundAttenuation`) null))))
        (:`then_1`
          (`SceneComponent.K2_SetRelativeRotation` _pendulum_pivot_2 (`KismetMathLibrary.MakeRotator` (.roll (.rotation _returnvalue_3)) 0.0 (.yaw (.rotation _returnvalue_3))) false false)
          (`KismetSystemLibrary.K2_PauseTimer` null "UpdateTime"))))))

(event `UpdateSpeed`
  ;[1 1 1] Update time
  (`self.UpdateTime`)
  (`KismetSystemLibrary.K2_SetTimer` null "UpdateTime" (/ 1.0 (`KismetMathLibrary.Conv_IntToDouble` (`self.Speed`))) true)
  (`TimelineComponent.SetPlayRate` (`self.MovePendulum`) (`KismetMathLibrary.Conv_IntToDouble` (`self.Speed`)))
  (goto _label))

(event `Bell Hour`
  ;[0.8071 1 0.04797] Sound
  (`KismetSystemLibrary.RetriggerableDelay` 2.0)
  (`GameplayStatics.SpawnSoundAttached` (`self.BellSound`) (`self.clock`) "None" (0.0 0.0 0.0) (struct) "KeepRelativeOffset" true (`self.Volume`) 1.0 0.0 (`self.SoundAttenuation`) null)
  (bind _output_get (set `self.BellNum` (- (`self.BellNum`) 1)))
  (if (> _output_get 0)
    (`self.Bell Hour`)))

(fn `Set Clock Hand`
  (params (sec :type Integer) (min :type Integer) (hour :type Integer))
  (bind (_output _return) (`self.PeriodReset` hour 13))
  (bind _returnvalue (+ (select `bool` (`self.OnlyMoveSec`) :`false` (/ (`KismetMathLibrary.Conv_IntToDouble` sec) 60.0)) (`KismetMathLibrary.Conv_IntToDouble` min)))
  ;[1 1 1] Set Clock
  (`SceneComponent.K2_SetRelativeRotation` (`self.Sec_pivot`) (`KismetMathLibrary.MakeRotator` 0.0 (`KismetMathLibrary.Conv_IntToDouble` (* sec -6))) false false)
  (`SceneComponent.K2_SetRelativeRotation` (`self.MIN_pivot`) (`KismetMathLibrary.MakeRotator` 0.0 (* -6 _returnvalue)) false false)
  (`SceneComponent.K2_SetRelativeRotation` (`self.H_pivot`) (`KismetMathLibrary.MakeRotator` 0.0 (* -30 (+ (select `bool` (`self.OnlyMoveSec`) :`false` (/ _returnvalue 60.0)) (`KismetMathLibrary.Conv_IntToDouble` hour)))) false false)
  (switch `/Game/VariousInteractiveClock/Blueprints/Enumeration/E_clock_bell` (`self.BellType`)
    (:`NewEnumerator0`
      ;[1 0 0.3634] The bell rings on the hour
      (if (and (== min 0) (== sec 0))
        (set `self.BellNum` (select `bool` _return :`false` _output :`true` (+ _output 1)))
        (`GameplayStatics.SpawnSoundAttached` "/Game/VariousInteractiveClock/Audio/Strike_the_clock_star_wav.Strike_the_clock_star_wav" (`self.clock`) "None" (0.0 0.0 0.0) (struct) "KeepRelativeOffset" true (`self.Volume`) 1.0 0.0 (`self.SoundAttenuation`) null)
        (`self.Bell Hour`)))
    (:`NewEnumerator1`
      ;[0 1 0.2751] Alarm Ring
      (if (and (== hour (`self.hour_alarm`)) (== min (`self.min_alarm`)) (== sec (`self.sec_alarm`)))
        (`GameplayStatics.SpawnSoundAttached` (`self.BellSound`) (`self.clock`) "None" (0.0 0.0 0.0) (struct) "KeepRelativeOffset" true (`self.Volume`) 1.0 0.0 (`self.SoundAttenuation`) null)))))

(fn `UpdateTime`
  (bind _returnvalue (`KismetMathLibrary.Now`))
  (bind (_returnvalue_year _returnvalue_month _returnvalue_day _returnvalue_hour _returnvalue_minute _returnvalue_second) (`KismetMathLibrary.BreakDateTime` (+ (`KismetMathLibrary.MakeDateTime` 2020 11 30 (`self.Hour`) (`self.Min`) (`self.Sec`)) (`KismetMathLibrary.MakeTimespan` 0 0 0 1))))
  ;[1 1 1] Clock
  (if (`self.OnlyMoveSec`)
    ;[1 0 0.02427] Only move the second hand
    (`self.Set Clock Hand` (`KismetMathLibrary.GetSecond` (`KismetMathLibrary.Now`)) (`self.min`) (`self.hour`))
    (elif (`self.SysTime`)
      ;[0.01812 1 0.3269] Get operating system time
      (`self.Set Clock Hand` (`KismetMathLibrary.GetSecond` _returnvalue) (`KismetMathLibrary.GetMinute` _returnvalue) (`KismetMathLibrary.GetHour12` _returnvalue))
      (else
        (`self.Set Clock Hand` _returnvalue_second _returnvalue_minute _returnvalue_hour)
        (set `self.Hour` _returnvalue_hour)
        (set `self.Min` _returnvalue_minute)
        (set `self.Sec` _returnvalue_second)))))

(fn `UserConstructionScript`
  (bind _pendulum_pivot (`self.pendulum_pivot`))
  (bind _returnvalue (`SceneComponent.GetRelativeTransform` _pendulum_pivot))
  (`parent.UserConstructionScript`)
  (`self.Upload`)
  (`SceneComponent.SetVisibility` (`self.second`) (`self.HasSecondHand`) true)
  (`SceneComponent.SetVisibility` (`self.clockBase`) (`self.HasClockBase`) true)
  (`SceneComponent.SetVisibility` (`self.pendulum`) (`self.HasPendulum`) true)
  (`SceneComponent.K2_SetRelativeRotation` _pendulum_pivot (`KismetMathLibrary.MakeRotator` (.roll (.rotation _returnvalue)) (`KismetMathLibrary.Conv_IntToDouble` (`self.Angle Pendulum`)) (.yaw (.rotation _returnvalue))) false false)
  (`TimelineComponent.SetNewTime` (`self.MovePendulum`) 0.5)
  (`|ExecutionSequence`
    (:`then_0`
      (if (not (`self.HasSecondHand`))
        (set `self.OnlyMoveSec` false)))
    (:`then_1`
      (if (`self.AutoWorking`)
        (if (`self.OnlyMoveSec`)
          (set `self.SysTime` false)
          (set `self.BellType` "NewEnumerator2"))
        (else
          (set `self.SysTime` false)
          (set `self.OnlyMoveSec` false)
          (set `self.BellType` "NewEnumerator2")
          (set `self.OnlyMoveSec` false)
          (set `self.InteractionEnabled` false))))
    (:`then_2`
      (if (not (`self.HasPendulum`))
        (set `self.Angle Pendulum` 0)))
    (:`then_3`
      (switch `/Game/VariousInteractiveClock/Blueprints/Enumeration/E_clock_bell` (`self.BellType`)
        (:`NewEnumerator0`
          _)
        (:`NewEnumerator2`
          _))
      (set `self.hour_alarm` 0)
      (set `self.min_alarm` 0)
      (set `self.sec_alarm` 0))))