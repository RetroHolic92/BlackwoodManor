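; Interactive digital clock that shows system time, counts up from a set time, or counts down to a bell and ClockEvent.
; A looping timer scaled by Speed runs UpdateTime, using DateTime math on a dummy date for rollover.
; Zero-padded values feed a screen widget.
; Use starts an inspection with a WI_function widget initialized to the current time fields, and alternative use closes it.
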(event `Upload`
  ;[1 1 1] Upload
  (`self.Set Clock Hand` (`self.Sec`) (`self.Min`) (`self.Hour`)))

(event `self.Use`
  (params (`XHC Event` :type Boolean))
  ;[1 0.04588 0] Child blueprint essential
  (`self.BeginInspection` (`self.Billboard`))
  (`UserWidget.AddToViewport` (`self.WI_function`) 100)
  (`/Game/VariousInteractiveClock/Widget/WI_function.ClockFocStart` (`self.WI_function`))
  (`/Game/VariousInteractiveClock/Widget/WI_function.Initial Time` (`self.WI_function`) (`self.Hour`) (`self.Min`) (`self.Sec`)))

(event `self.InspectionAlternativeUse`
  ;[1 0.04588 0] Child blueprint essential
  (`/Game/VariousInteractiveClock/Widget/WI_function.ClockFocStop` (`self.WI_function`))
  (`KismetSystemLibrary.Delay` 0.5)
  (`self.EndInspection` false)
  (`Widget.RemoveFromParent` (`self.WI_function`)))

(event `self.ReceiveBeginPlay`
  ;[0 0.2676 1] Clock screen
  (bind _returnvalue (`|CreateWidget` "/Game/VariousInteractiveClock/Widget/WI_clock_screen.WI_clock_screen_C" null (`self.HasSecondNum`)))
  (bind _output_get (set `self.Secret_screen` _returnvalue))
  (`WidgetComponent.SetWidget` (`self.screen`) _output_get)
  (`KismetSystemLibrary.Delay` 0.01)
  (`self.update`)
  (bind _returnvalue_2 (`|CreateWidget` "/Game/VariousInteractiveClock/Widget/WI_function.WI_function_C" null self))
  (bind _output_get_2 (set `self.WI_function` _returnvalue_2))
  (`WidgetComponent.SetWidget` (`self.function`) _output_get_2)
  (`SceneComponent.SetVisibility` (`self.function`) false true))

(event `UpDate`
  (bind _returnvalue (`KismetMathLibrary.Now`))
  ;[1 1 1] Update time
  (if (`self.AutoWorking`)
    (set `self.0_hour` (- (`self.Hour`) (`KismetMathLibrary.GetHour` _returnvalue)))
    (set `self.0_min` (- (`self.Min`) (`KismetMathLibrary.GetMinute` _returnvalue)))
    (set `self.0_sec` (- (`self.Sec`) (`KismetMathLibrary.GetSecond` _returnvalue)))
    (`self.UpdateSpeed`)
    (else
      (`self.Set Clock Hand` (`self.Hour`) (`self.Min`) (`self.Hour`)))))

(event `UpdateSpeed`
  ;[1 1 1] Update time
  (`self.UpdateTime`)
  (`KismetSystemLibrary.K2_SetTimer` null "UpdateTime" (/ 1.0 (`KismetMathLibrary.Conv_IntToDouble` (`self.Speed`))) true))

(event `Bell`
  ;[1 0.8704 0] Sound
  (`GameplayStatics.SpawnSoundAttached` (`self.BellSound`) (`self.clock`) "None" (0.0 0.0 0.0) (struct) "KeepRelativeOffset" true (`self.Volume`) 1.0 0.0 (`self.SoundAttenuation`) null))

(event `ClockEvent`)

(fn `Add 0`
  (params (time :type Integer))
  (returns (time_add_0 :type String))
  (return (select `bool` (< time 10) :`false` (`KismetStringLibrary.Conv_IntToString` time) :`true` (`KismetStringLibrary.Concat_StrStr` "0" (`KismetStringLibrary.Conv_IntToString` time)))))

(fn `Set Clock Hand`
  (params (sec :type Integer) (min :type Integer) (hour :type Integer))
  (bind _time_add_0 (`self.Add 0` sec))
  (bind _time_add_0_2 (`self.Add 0` min))
  (bind _time_add_0_3 (`self.Add 0` hour))
  (`/Game/VariousInteractiveClock/Widget/WI_clock_screen.update screen` :`self` (`self.Secret_screen`) :`h` _time_add_0_3 :`min` _time_add_0_2 :`sec` _time_add_0))

(fn `UpdateTime`
  (bind _returnvalue (`KismetMathLibrary.Now`))
  (bind (_returnvalue_year _returnvalue_month _returnvalue_day _returnvalue_hour _returnvalue_minute _returnvalue_second) (`KismetMathLibrary.BreakDateTime` (+ (`KismetMathLibrary.MakeDateTime` 2020 11 30 (`self.Hour`) (`self.Min`) (`self.Sec`)) (`KismetMathLibrary.MakeTimespan` 0 0 0 1))))
  (bind (_returnvalue_year_2 _returnvalue_month_2 _returnvalue_day_2 _returnvalue_hour_2 _returnvalue_minute_2 _returnvalue_second_2) (`KismetMathLibrary.BreakDateTime` (+ (`KismetMathLibrary.MakeDateTime` 2020 11 30 (`self.Hour`) (`self.Min`) (`self.Sec`)) (`KismetMathLibrary.MakeTimespan` 0 0 0 -1))))
  ;[1 1 1] Clock
  (if (`self.pause`)
    _
    (elif (`self.SysTime`)
      (`self.Set Clock Hand` (`KismetMathLibrary.GetSecond` _returnvalue) (`KismetMathLibrary.GetMinute` _returnvalue) (`KismetMathLibrary.GetHour` _returnvalue))
      (elif (`self.Countdown`)
        ;[0 1 0.6481] Countdown
        (`self.Set Clock Hand` _returnvalue_second_2 _returnvalue_minute_2 _returnvalue_hour_2)
        (bind _output_get (set `self.Hour` _returnvalue_hour_2))
        (bind _output_get_2 (set `self.Min` _returnvalue_minute_2))
        (bind _output_get_3 (set `self.Sec` _returnvalue_second_2))
        (if (and (== _output_get_3 0) (== _output_get_2 0) (== _output_get 0))
          (`self.Bell`)
          (`KismetSystemLibrary.K2_PauseTimer` null "UpdateTime")
          (`self.ClockEvent`))
        (else
          (`self.Set Clock Hand` _returnvalue_second _returnvalue_minute _returnvalue_hour)
          (set `self.Hour` _returnvalue_hour)
          (set `self.Min` _returnvalue_minute)
          (set `self.Sec` _returnvalue_second))))))

(fn `UserConstructionScript`
  (`parent.UserConstructionScript`)
  (`self.Upload`)
  (if (`self.AutoWorking`)
    (if (`self.Countdown`)
      (set `self.SysTime` false))
    (else
      (set `self.SysTime` false)
      (set `self.Countdown` false)
      (set `self.InteractionEnabled` false))))